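; Minimap bounds trigger that controls which actors' icons show on the minimap, using a sphere or box volume to match its shape.
; Overlaps from "MinimapCollision"-tagged actors add or remove their attach parent's icon component on the widget, with enabled and in-area checks on show (player skips area check).
; Actors arriving before the minimap initialises are queued and rechecked by looping timer.
; Tick zeroes rotation so the box stays world-aligned.
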(event OnComponentBeginOverlap(Box_Trigger)
  (params (OverlappedComponent :type Primitive%20Component%20Object%20Reference) (OtherActor :type Actor%20Object%20Reference) (OtherComp :type Primitive%20Component%20Object%20Reference) (OtherBodyIndex :type Integer) (bFromSweep :type Boolean) (SweepResult :type Hit%20Result%20Structure%20%28by%20ref%29))
  ;[1 1 1] The minimap can be circle or square.
  ; The appropriate trigger checks actors that come within
  ; range to be displayed on the minimap.
  (CallFunction|CheckActorValid OtherActor))

(event OnComponentEndOverlap(Box_Trigger)
  (params (OverlappedComponent :type Primitive%20Component%20Object%20Reference) (OtherActor :type Actor%20Object%20Reference) (OtherComp :type Primitive%20Component%20Object%20Reference) (OtherBodyIndex :type Integer))
  ;[1 1 1] When an actor has left the trigger, check if they should be hidden
  (CallFunction|CheckSetActorHide OtherActor))

(event OnComponentBeginOverlap(Sphere_Trigger)
  (params (OverlappedComponent :type Primitive%20Component%20Object%20Reference) (OtherActor :type Actor%20Object%20Reference) (OtherComp :type Primitive%20Component%20Object%20Reference) (OtherBodyIndex :type Integer) (bFromSweep :type Boolean) (SweepResult :type Hit%20Result%20Structure%20%28by%20ref%29))
  ;[1 1 1] The minimap can be circle or square.
  ; The appropriate trigger checks actors that come within
  ; range to be displayed on the minimap.
  (CallFunction|CheckActorValid OtherActor))

(event OnComponentEndOverlap(Sphere_Trigger)
  (params (OverlappedComponent :type Primitive%20Component%20Object%20Reference) (OtherActor :type Actor%20Object%20Reference) (OtherComp :type Primitive%20Component%20Object%20Reference) (OtherBodyIndex :type Integer))
  ;[1 1 1] When an actor has left the trigger, check if they should be hidden
  (CallFunction|CheckSetActorHide OtherActor))

(event Custom|CheckSetActorShow
  (params (Actor :type Actor%20Object%20Reference))
  (bind _returnvalue (Actor|GetAttachParentActor Actor))
  (bind _returnvalue_2 (Actor|GetComponentbyClass _returnvalue "/Game/Minimap/Blueprints/Component_MinimapIcon.Component_MinimapIcon_C"))
  ;[1 1 1] Check again if the actor is overlapping the trigger (in case they exited while waiting for the minimap to become active).
  ; If they are inside the visibility trigger, need to also check if they are within the minimap bounds.
  ; If so, activate their minimap icon and add them to the minimap to be shown.
  (Utilities|IsValid Actor
    (:Is%20Valid
      (Utilities|IsValid _returnvalue
        (:Is%20Valid
          (if (CallFunction|IsOverlapping Actor)
            (if (or (Default|IsActorInsideMinimapArea (Variables|/Game/Minimap/Blueprints/Widgets/Widget_Minimap.Widget_Minimap_C|GetMinimapObject (Variables|Default|GetMinimapWidget)) Actor) (== _returnvalue (CallFunction|BPFLGetPlayer)))
              (if (Variables|/Game/Minimap/Blueprints/Component_MinimapIcon.Component_MinimapIcon_C|GetIconsEnabled _returnvalue_2)
                (Default|AddActortoShow (Variables|Default|GetMinimapWidget) _returnvalue_2)))))))))

(event Custom|CheckSetActorHide
  (params (Actor :type Actor%20Object%20Reference))
  (bind _returnvalue (Actor|GetAttachParentActor Actor))
  ;[1 1 1] Checks the actor that left the trigger is a valid minimap object.
  ; If so, deactivate it, and remove the actor from the minimap widget.
  (if (Actor|ActorHasTag Actor "MinimapCollision")
    (Utilities|IsValid _returnvalue
      (:Is%20Valid
        (Default|RemoveActortoShow (Variables|Default|GetMinimapWidget) (Actor|GetComponentbyClass _returnvalue "/Game/Minimap/Blueprints/Component_MinimapIcon.Component_MinimapIcon_C"))))))

(event Custom|CheckMinimapValid
  (bind _minimapwidget (Variables|Default|GetMinimapWidget))
  (bind _minimapobject (Variables|/Game/Minimap/Blueprints/Widgets/Widget_Minimap.Widget_Minimap_C|GetMinimapObject _minimapwidget))
  ;[1 1 1] When the minimap becomes valid, add any actors to it
  ; that were waiting for the minimap to become initialised.
  ; This is a repeating function on a timer, so once the minimap is valid, kill the timer.
  (Utilities|IsValid _minimapwidget
    (:Is%20Valid
      (Utilities|IsValid _minimapobject
        (:Is%20Valid
          (if (Variables|/Game/Minimap/Blueprints/BP_Minimap.BP_Minimap_C|GetINTERNAL_IsInitialised _minimapobject)
            (Utilities|Time|ClearandInvalidateTimerbyHandle (Variables|Default|GetCheckMinimapValidTimerHandle))
            (for _array_element (Variables|Default|GetListOfActorsToRepeatedlyCheckForValidity)
              (CallFunction|CheckSetActorShow _array_element))))))))

(event Custom|CheckActorValid
  (params (Actor :type Actor%20Object%20Reference))
  (bind _minimapwidget (Variables|Default|GetMinimapWidget))
  (bind _minimapobject (Variables|/Game/Minimap/Blueprints/Widgets/Widget_Minimap.Widget_Minimap_C|GetMinimapObject _minimapwidget))
  ;[1 1 1] Checks if actors that enter the trigger are valid actors to be shown on the minimap.
  ; If so, checks that the actual minimap is valid and ready to accept actors to be shown on it. If so, add the actor to the minimap to be shown.
  ; If not, add them temporarily to an array, then repeatedly check when the minimap is ready and initialised, and add them at that point.
  (if (Actor|ActorHasTag Actor "MinimapCollision")
    (Utilities|IsValid _minimapwidget
      (:Is%20Valid
        (Utilities|IsValid _minimapobject
          (:Is%20Valid
            (if (Variables|/Game/Minimap/Blueprints/BP_Minimap.BP_Minimap_C|GetINTERNAL_IsInitialised _minimapobject)
              (CallFunction|CheckSetActorShow Actor)
              (else
                (Utilities|Array|Add (Variables|Default|GetListOfActorsToRepeatedlyCheckForValidity) Actor :!label _label)
                (bind _returnvalue (Utilities|Time|SetTimerbyEvent (EventDispatchers|CreateEvent :!event Custom|CheckMinimapValid) 0.05 true))
                (Variables|Default|SetCheckMinimapValidTimerHandle _returnvalue))))
          (:Is%20Not%20Valid
            (goto _label))))
      (:Is%20Not%20Valid
        (goto _label)))))

(event EventTick
  (params (DeltaSeconds :type Float%20%28single-precision%29))
  ;[1 1 1] Clear the rotation. This is required for the Box trigger only, because
  ; it is attached to the player (if set to move/scroll) and will rotate with them.
  (Transformation|SetActorRotation "0, 0, 0"))

(event EventBeginPlay
  ;[1 1 1] Store a copy of the minimap widget
  (bind _foundwidgets (Widget|GetAllWidgetsOfClass "/Game/Minimap/Blueprints/Widgets/Widget_Minimap.Widget_Minimap_C" true))
  (if (> (Utilities|Array|Length _foundwidgets) 0)
    (Variables|Default|SetMinimapWidget (Utilities|Array|Get(acopy) _foundwidgets))))

(fn ConstructionScript)

(fn SetTriggerShape
  (params (MinimapShape :type ENUM_MinimapShape%20Enum :default "NewEnumerator0") (VisibilityDistance :type Float%20%28single-precision%29) (VisibilityHeight :type Float%20%28single-precision%29) (Enabled :type Boolean))
  ;[1 1 1] Sets the trigger shape, and updates the size based on supplied parameters.
  ; Also enables tick if the shape is square, since it needs to have its rotation zeroed each tick.
  (if Enabled
    (Variables|Default|SetMinimapShape MinimapShape)
    (if (Utilities|Enum|Equal(Enum) (Variables|Default|GetMinimapShape) "NewEnumerator0")
      (Collision|SetCollisionEnabled (Variables|Default|GetSphere_Trigger) "QueryOnly")
      (Components|Sphere|SetSphereRadius (Variables|Default|GetSphere_Trigger) VisibilityDistance true)
      (else
        (Collision|SetCollisionEnabled (Variables|Default|GetBox_Trigger) "QueryOnly")
        (Components|Box|SetBoxExtent (Variables|Default|GetBox_Trigger) (Math|Vector|MakeVector VisibilityDistance VisibilityDistance VisibilityHeight) true)
        (Actor|Tick|SetActorTickEnabled true)))
    (else
      ;[1 1 1] Disable collision and tick, if this trigger is set to disabled.
      (Collision|SetCollisionEnabled (Variables|Default|GetSphere_Trigger) "NoCollision")
      (Actor|Tick|SetActorTickEnabled false))))

(fn IsOverlapping
  (params (OtherActor :type Actor%20Object%20Reference))
  ;[1 1 1] Checks if the actor is overlapping this trigger, based on this trigger's shape.
  (switch Utilities|FlowControl|Switch|SwitchonENUM_MinimapShape (Variables|Default|GetMinimapShape)
    (:NewEnumerator0
      (return (Collision|IsOverlappingActor (Variables|Default|GetSphere_Trigger) OtherActor :!class /Script/Engine.PrimitiveComponent)))
    (:NewEnumerator1
      (return (Collision|IsOverlappingActor (Variables|Default|GetBox_Trigger) OtherActor :!class /Script/Engine.PrimitiveComponent)))))