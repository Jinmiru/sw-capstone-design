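; BP_TreasureChest is a minimap demo chest that opens when the player walks into it and drops off the minimap.
; The trigger box overlap checks for the player, starts the opening, disables its own collision and changes the minimap icon component's state to permanently remove the icon.
; A timeline drives the lid mesh's pitch to animate the opening.
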(event OnComponentBeginOverlap(Box_Trigger)
  (params (OverlappedComponent :type Primitive%20Component%20Object%20Reference) (OtherActor :type Actor%20Object%20Reference) (OtherComp :type Primitive%20Component%20Object%20Reference) (OtherBodyIndex :type Integer) (bFromSweep :type Boolean) (SweepResult :type Hit%20Result%20Structure%20%28by%20ref%29))
  ;[1 1 1] If player walks up to treasure chest, open the lid and remove from the minimap (icon destroyed forever)
  (if (== OtherActor (CallFunction|BPFLGetPlayer))
    (CallFunction|OpenChest)
    (Collision|SetCollisionEnabled (Variables|Default|GetBox_Trigger) "NoCollision")
    (Default|SetState (Variables|Default|GetComponent_MinimapIcon) "NewEnumerator2")))

(event Custom|OpenChest
  (bind _sm_treasurechestlid (Variables|Default|GetSM_TreasureChestLid))
  ;[1 1 1] Open lid animation
  (bind _lidangle (Timeline|OpenLid Play)
    (:Update
      (Transformation|SetRelativeLocationAndRotation _sm_treasurechestlid (Variables|/Script/Engine.SceneComponent|GetRelativeLocation _sm_treasurechestlid) (Math|Rotator|MakeRotator 0.0 _lidangle 0.0) true true))))

(fn ConstructionScript)