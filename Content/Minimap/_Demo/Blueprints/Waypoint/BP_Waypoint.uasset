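; BP_Waypoint is a demo waypoint actor that routes NPCs along their waypoint lists.
; When a BP_Npc_Base enters its trigger sphere and this waypoint is that NPC's next target, it tells the NPC to prepare the following waypoint.
; The construction script writes the waypoint's ID to a text render component as an editor label, hidden at runtime.
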(event OnComponentBeginOverlap(Sphere_Trigger)
  (params (OverlappedComponent :type Primitive%20Component%20Object%20Reference) (OtherActor :type Actor%20Object%20Reference) (OtherComp :type Primitive%20Component%20Object%20Reference) (OtherBodyIndex :type Integer) (bFromSweep :type Boolean) (SweepResult :type Hit%20Result%20Structure%20%28by%20ref%29))
  ;[1 1 1] If NPC walks into this waypoint, send them to the next one in their waypoint list
  (bind _asbp_npc_base (Utilities|Casting|CastToBP_Npc_Base OtherActor))
  (if (== (Default|GetNextWaypoint _asbp_npc_base) self)
    (Default|PrepareNextWaypoint _asbp_npc_base)))

(fn ConstructionScript
  ;[1 1 1] Set the ID text in editor (hidden during runtime)
  (Rendering|Components|TextRender|SetText (Variables|Default|GetTextRender_ID) (Utilities|Text|ToText(Integer) (Variables|Default|GetID))))