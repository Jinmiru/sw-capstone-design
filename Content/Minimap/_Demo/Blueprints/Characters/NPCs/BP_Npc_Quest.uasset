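; Minimap demo quest NPC that simulates a player accepting and completing a quest through its minimap and in-world icons.
; The icon defaults to an exclamation mark, or starts as a question mark when IsQuestionMark is set.
; When the player overlaps Box_Trigger, an exclamation mark becomes a question mark, while an existing question mark changes the ComponentMinimapIcon state to remove both icons.
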(event OnComponentBeginOverlap(Box_Trigger)
  (params (OverlappedComponent :type Primitive%20Component%20Object%20Reference) (OtherActor :type Actor%20Object%20Reference) (OtherComp :type Primitive%20Component%20Object%20Reference) (OtherBodyIndex :type Integer) (bFromSweep :type Boolean) (SweepResult :type Hit%20Result%20Structure%20%28by%20ref%29))
  ;[1 1 1] When the player gets close to the quest NPC;
  ; - If the icon is currently an exclamation mark, simulate the player accepting the quest and change it to a question mark.
  ; - If the icon is currently a question mark, simulate the player completing the quest and destroy both the minimap and in world icons.
  (if (== OtherActor (CallFunction|BPFLGetPlayer))
    (if (Variables|Default|GetIsQuestionMark)
      (Default|SetState (Variables|Default|GetComponent_MinimapIcon) "NewEnumerator2")
      (else
        (CallFunction|SetQuestionMark)
        (Variables|Default|SetIsQuestionMark true)))))

(event Custom|SetQuestionMark
  (bind _component_minimapicon (Variables|Default|GetComponent_MinimapIcon))
  ;[1 1 1] Set both the minimap and in world icon to a question mark
  (Default|SetMinimapImage _component_minimapicon "/Game/Minimap/Textures/MinimapIcons/T_QuestionMark.T_QuestionMark")
  (Default|SetinWorldImage _component_minimapicon "/Game/Minimap/Textures/MinimapIcons/T_QuestionMarkBig.T_QuestionMarkBig"))

(event EventBeginPlay
  ;[1 1 1] By default the icon is an exclamation mark.
  ; If question mark is set to true, then on start, change the icon to a question mark.
  (if (Variables|Default|GetIsQuestionMark)
    (CallFunction|SetQuestionMark)))

(fn ConstructionScript)