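; BP_GamePlayerController is the InventoryKit player controller, caching the controlled Character and tracking the currently available interaction type.
; InitializePlayer runs on BeginPlay for the local controller and again on Possess to refresh that Character reference.
; BeginPlay also has the Game Instance display a game widget message.
; Helper functions get or update the interaction type and branch on whether the controlled pawn is valid and locally controlled.
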(event EventBeginPlay
  ;[1 1 1 1 16] Begin Play
  ;;[1 1 1 1 16] Initialize The Player
  (if (Pawn|IsLocalController)
    (CallFunction|InitializePlayer)
    ;;[1 1 1 1 16] To Keep Things In Game Instance
    (Class|BPGameInstanceInterface|DisplayGameWidget(Message) (Game|GetGameInstance) "NewEnumerator3")))

(event EventPossess
  (params (PossessedPawn :type Pawn%20Object%20Reference))
  ;[1 1 1 1 16] Re-Init On Possess
  (CallFunction|InitializePlayer))

(fn ConstructionScript)

(fn InitializePlayer
  (bind _ascharacter (Utilities|Casting|CastToCharacter (Pawn|GetControlledPawn)))
  (Variables|Components|SetControlledCharacter _ascharacter))

(fn GetAvailableInteractionType
  (return (Variables|Default|GetAvailableInteractionType)))

(fn UpdateAvailableInteractionType
  (params (InteractionType :type Enum_InteractionType%20Enum :default "NewEnumerator0"))
  (Variables|Default|SetAvailableInteractionType InteractionType)
  (return true))