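; Blueprint function library for the portals VFX pack, providing helpers that play mesh dissolve and spawn effects and rotate a VR pawn.
; Effect functions attach auto-destroying Niagara systems and pass in portal and mesh locations, color, size and axes.
; Static and skeletal meshes have standard and VR variants, and dissolves also offer a sphere version.
; The pawn helper rotates the actor, then offsets it to compensate for camera displacement.
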(fn FunctRotateVRPawn
  (params (VRPawn :type Actor%20Object%20Reference) (CurrentRotation :type Rotator) (NewRotation :type Rotator))
  (bind _output_get (LocalVariables|SetVR_Pawn VRPawn))
  (LocalVariables|SetCamera (Actor|GetComponentbyClass _output_get "/Script/Engine.CameraComponent"))
  (LocalVariables|SetAddRotation (Math|Rotator|Delta(Rotator) NewRotation CurrentRotation))
  (LocalVariables|SetDeltaLocation (- (Transformation|GetWorldLocation (LocalVariables|GetCamera)) (Math|Transform|TransformLocation (Math|Transform|MakeTransform (.Location (Math|Transform|BreakTransform (Transformation|GetActorTransform (LocalVariables|GetVR_Pawn)))) (Math|Rotator|CombineRotators (.Rotation (Math|Transform|BreakTransform (Transformation|GetActorTransform (LocalVariables|GetVR_Pawn)))) (LocalVariables|GetAddRotation)) (.Scale (Math|Transform|BreakTransform (Transformation|GetActorTransform (LocalVariables|GetVR_Pawn))))) (Variables|/Script/Engine.SceneComponent|GetRelativeLocation (LocalVariables|GetCamera)))))
  (Class|Actor|AddActorWorldRotation (LocalVariables|GetVR_Pawn) (LocalVariables|GetAddRotation))
  (Transformation|AddActorWorldOffset (LocalVariables|GetVR_Pawn) (LocalVariables|GetDeltaLocation)))

(fn FunctDissolveSkMesh
  (params (bSphere? :type Boolean) (AttachToComponent :type Scene%20Component%20Object%20Reference) (PortalLocation :type Vector) (MeshLocation :type Vector) (Color :type Linear%20Color%20Structure) (Size :type Float%20%28double-precision%29) (Xaxis :type Vector) (Yaxis :type Vector) (Zaxis :type Vector))
  (if (not bSphere?)
    (bind _returnvalue (Niagara|SpawnSystemAttached "/Game/Portals_VFXPack/Particles/P_DissolveSkMesh.P_DissolveSkMesh" AttachToComponent "None" "0, 0, 0" "0, 0, 0" "KeepRelativeOffset" true))
    (Effects|Components|ParticleSystem|SetVectorParameter _returnvalue "User.EndLocation" PortalLocation)
    (Effects|Components|ParticleSystem|SetVectorParameter _returnvalue "User.StartLocation" MeshLocation)
    (Effects|Components|ParticleSystem|SetColorParameter _returnvalue "User.Color" Color)
    (Effects|Components|ParticleSystem|SetFloatParameter _returnvalue "User.Size" Size)
    (Effects|Components|ParticleSystem|SetVectorParameter _returnvalue "User.Xaxis" Xaxis)
    (Effects|Components|ParticleSystem|SetVectorParameter _returnvalue "User.Yaxis" Yaxis)
    (Effects|Components|ParticleSystem|SetVectorParameter _returnvalue "User.Zaxis" Zaxis)
    (else
      (bind _returnvalue_2 (Niagara|SpawnSystemAttached "/Game/Portals_VFXPack/Particles/P_DissolveSkMeshSphere.P_DissolveSkMeshSphere" AttachToComponent "None" "0, 0, 0" "0, 0, 0" "KeepRelativeOffset" true))
      (Effects|Components|ParticleSystem|SetVectorParameter _returnvalue_2 "User.EndLocation" PortalLocation)
      (Effects|Components|ParticleSystem|SetVectorParameter _returnvalue_2 "User.StartLocation" MeshLocation)
      (Effects|Components|ParticleSystem|SetColorParameter _returnvalue_2 "User.Color" Color)
      (Effects|Components|ParticleSystem|SetFloatParameter _returnvalue_2 "User.Size" Size)
      (Effects|Components|ParticleSystem|SetVectorParameter _returnvalue_2 "User.Xaxis" Xaxis)
      (Effects|Components|ParticleSystem|SetVectorParameter _returnvalue_2 "User.Yaxis" Yaxis)
      (Effects|Components|ParticleSystem|SetVectorParameter _returnvalue_2 "User.Zaxis" Zaxis))))

(fn FunctDissolveStMesh
  (params (bSphere? :type Boolean) (AttachToComponent :type Scene%20Component%20Object%20Reference) (PortalLocation :type Vector) (MeshLocation :type Vector) (Color :type Linear%20Color%20Structure) (Size :type Float%20%28double-precision%29) (Xaxis :type Vector) (Yaxis :type Vector) (Zaxis :type Vector))
  (if (not bSphere?)
    (bind _returnvalue (Niagara|SpawnSystemAttached "/Game/Portals_VFXPack/Particles/P_DissolveStMesh.P_DissolveStMesh" AttachToComponent "None" "0, 0, 0" "0, 0, 0" "KeepRelativeOffset" true))
    (Effects|Components|ParticleSystem|SetVectorParameter _returnvalue "User.EndLocation" PortalLocation)
    (Effects|Components|ParticleSystem|SetVectorParameter _returnvalue "User.StartLocation" MeshLocation)
    (Effects|Components|ParticleSystem|SetColorParameter _returnvalue "User.Color" Color)
    (Effects|Components|ParticleSystem|SetFloatParameter _returnvalue "User.Size" Size)
    (Effects|Components|ParticleSystem|SetVectorParameter _returnvalue "User.Xaxis" Xaxis)
    (Effects|Components|ParticleSystem|SetVectorParameter _returnvalue "User.Yaxis" Yaxis)
    (Effects|Components|ParticleSystem|SetVectorParameter _returnvalue "User.Zaxis" Zaxis)
    (else
      (bind _returnvalue_2 (Niagara|SpawnSystemAttached "/Game/Portals_VFXPack/Particles/P_DissolveStMeshSphere.P_DissolveStMeshSphere" AttachToComponent "None" "0, 0, 0" "0, 0, 0" "KeepRelativeOffset" true))
      (Effects|Components|ParticleSystem|SetVectorParameter _returnvalue_2 "User.EndLocation" PortalLocation)
      (Effects|Components|ParticleSystem|SetVectorParameter _returnvalue_2 "User.StartLocation" MeshLocation)
      (Effects|Components|ParticleSystem|SetColorParameter _returnvalue_2 "User.Color" Color)
      (Effects|Components|ParticleSystem|SetFloatParameter _returnvalue_2 "User.Size" Size)
      (Effects|Components|ParticleSystem|SetVectorParameter _returnvalue_2 "User.Xaxis" Xaxis)
      (Effects|Components|ParticleSystem|SetVectorParameter _returnvalue_2 "User.Yaxis" Yaxis)
      (Effects|Components|ParticleSystem|SetVectorParameter _returnvalue_2 "User.Zaxis" Zaxis))))

(fn FunctSpawnStMesh
  (params (AttachToComponent :type Scene%20Component%20Object%20Reference) (PortalLocation :type Vector) (MeshLocation :type Vector) (Color :type Linear%20Color%20Structure) (Size :type Float%20%28double-precision%29) (Xaxis :type Vector) (Yaxis :type Vector) (Zaxis :type Vector))
  (bind _returnvalue (Niagara|SpawnSystemAttached "/Game/Portals_VFXPack/Particles/P_SpawnStMesh.P_SpawnStMesh" AttachToComponent "None" "0, 0, 0" "0, 0, 0" "KeepRelativeOffset" true))
  (Effects|Components|ParticleSystem|SetVectorParameter _returnvalue "User.EndLocation" PortalLocation)
  (Effects|Components|ParticleSystem|SetVectorParameter _returnvalue "User.StartLocation" MeshLocation)
  (Effects|Components|ParticleSystem|SetColorParameter _returnvalue "User.Color" Color)
  (Effects|Components|ParticleSystem|SetFloatParameter _returnvalue "User.Size" Size)
  (Effects|Components|ParticleSystem|SetVectorParameter _returnvalue "User.Xaxis" Xaxis)
  (Effects|Components|ParticleSystem|SetVectorParameter _returnvalue "User.Yaxis" Yaxis)
  (Effects|Components|ParticleSystem|SetVectorParameter _returnvalue "User.Zaxis" Zaxis))

(fn FunctSpawnSkMesh
  (params (AttachToComponent :type Scene%20Component%20Object%20Reference) (PortalLocation :type Vector) (MeshLocation :type Vector) (Color :type Linear%20Color%20Structure) (Size :type Float%20%28double-precision%29) (Xaxis :type Vector) (Yaxis :type Vector) (Zaxis :type Vector))
  (bind _returnvalue (Niagara|SpawnSystemAttached "/Game/Portals_VFXPack/Particles/P_SpawnSkMesh.P_SpawnSkMesh" AttachToComponent "None" "0, 0, 0" "0, 0, 0" "KeepRelativeOffset" true))
  (Effects|Components|ParticleSystem|SetVectorParameter _returnvalue "User.EndLocation" PortalLocation)
  (Effects|Components|ParticleSystem|SetVectorParameter _returnvalue "User.StartLocation" MeshLocation)
  (Effects|Components|ParticleSystem|SetColorParameter _returnvalue "User.Color" Color)
  (Effects|Components|ParticleSystem|SetFloatParameter _returnvalue "User.Size" Size)
  (Effects|Components|ParticleSystem|SetVectorParameter _returnvalue "User.Xaxis" Xaxis)
  (Effects|Components|ParticleSystem|SetVectorParameter _returnvalue "User.Yaxis" Yaxis)
  (Effects|Components|ParticleSystem|SetVectorParameter _returnvalue "User.Zaxis" Zaxis))

(fn FunctDissolveSkMeshVR
  (params (bSphere? :type Boolean) (AttachToComponent :type Scene%20Component%20Object%20Reference) (PortalLocation :type Vector) (MeshLocation :type Vector) (Color :type Linear%20Color%20Structure) (Size :type Float%20%28double-precision%29) (Xaxis :type Vector) (Yaxis :type Vector) (Zaxis :type Vector))
  (if (not bSphere?)
    (bind _returnvalue (Niagara|SpawnSystemAttached "/Game/Portals_VFXPack/VR/Particles/P_VR_DissolveSkMesh.P_VR_DissolveSkMesh" AttachToComponent "None" "0, 0, 0" "0, 0, 0" "KeepRelativeOffset" true))
    (Effects|Components|ParticleSystem|SetVectorParameter _returnvalue "User.EndLocation" PortalLocation)
    (Effects|Components|ParticleSystem|SetVectorParameter _returnvalue "User.StartLocation" MeshLocation)
    (Effects|Components|ParticleSystem|SetColorParameter _returnvalue "User.Color" Color)
    (Effects|Components|ParticleSystem|SetFloatParameter _returnvalue "User.Size" Size)
    (Effects|Components|ParticleSystem|SetVectorParameter _returnvalue "User.Xaxis" Xaxis)
    (Effects|Components|ParticleSystem|SetVectorParameter _returnvalue "User.Yaxis" Yaxis)
    (Effects|Components|ParticleSystem|SetVectorParameter _returnvalue "User.Zaxis" Zaxis)
    (else
      (bind _returnvalue_2 (Niagara|SpawnSystemAttached "/Game/Portals_VFXPack/VR/Particles/P_VR_DissolveSkMeshSphere.P_VR_DissolveSkMeshSphere" AttachToComponent "None" "0, 0, 0" "0, 0, 0" "KeepRelativeOffset" true))
      (Effects|Components|ParticleSystem|SetVectorParameter _returnvalue_2 "User.EndLocation" PortalLocation)
      (Effects|Components|ParticleSystem|SetVectorParameter _returnvalue_2 "User.StartLocation" MeshLocation)
      (Effects|Components|ParticleSystem|SetColorParameter _returnvalue_2 "User.Color" Color)
      (Effects|Components|ParticleSystem|SetFloatParameter _returnvalue_2 "User.Size" Size)
      (Effects|Components|ParticleSystem|SetVectorParameter _returnvalue_2 "User.Xaxis" Xaxis)
      (Effects|Components|ParticleSystem|SetVectorParameter _returnvalue_2 "User.Yaxis" Yaxis)
      (Effects|Components|ParticleSystem|SetVectorParameter _returnvalue_2 "User.Zaxis" Zaxis))))

(fn FunctDissolveStMeshVR
  (params (bSphere? :type Boolean) (AttachToComponent :type Scene%20Component%20Object%20Reference) (PortalLocation :type Vector) (MeshLocation :type Vector) (Color :type Linear%20Color%20Structure) (Size :type Float%20%28double-precision%29) (Xaxis :type Vector) (Yaxis :type Vector) (Zaxis :type Vector))
  (if (not bSphere?)
    (bind _returnvalue (Niagara|SpawnSystemAttached "/Game/Portals_VFXPack/VR/Particles/P_VR_DissolveStMesh.P_VR_DissolveStMesh" AttachToComponent "None" "0, 0, 0" "0, 0, 0" "KeepRelativeOffset" true))
    (Effects|Components|ParticleSystem|SetVectorParameter _returnvalue "User.EndLocation" PortalLocation)
    (Effects|Components|ParticleSystem|SetVectorParameter _returnvalue "User.StartLocation" MeshLocation)
    (Effects|Components|ParticleSystem|SetColorParameter _returnvalue "User.Color" Color)
    (Effects|Components|ParticleSystem|SetFloatParameter _returnvalue "User.Size" Size)
    (Effects|Components|ParticleSystem|SetVectorParameter _returnvalue "User.Xaxis" Xaxis)
    (Effects|Components|ParticleSystem|SetVectorParameter _returnvalue "User.Yaxis" Yaxis)
    (Effects|Components|ParticleSystem|SetVectorParameter _returnvalue "User.Zaxis" Zaxis)
    (else
      (bind _returnvalue_2 (Niagara|SpawnSystemAttached "/Game/Portals_VFXPack/VR/Particles/P_VR_DissolveStMeshSphere.P_VR_DissolveStMeshSphere" AttachToComponent "None" "0, 0, 0" "0, 0, 0" "KeepRelativeOffset" true))
      (Effects|Components|ParticleSystem|SetVectorParameter _returnvalue_2 "User.EndLocation" PortalLocation)
      (Effects|Components|ParticleSystem|SetVectorParameter _returnvalue_2 "User.StartLocation" MeshLocation)
      (Effects|Components|ParticleSystem|SetColorParameter _returnvalue_2 "User.Color" Color)
      (Effects|Components|ParticleSystem|SetFloatParameter _returnvalue_2 "User.Size" Size)
      (Effects|Components|ParticleSystem|SetVectorParameter _returnvalue_2 "User.Xaxis" Xaxis)
      (Effects|Components|ParticleSystem|SetVectorParameter _returnvalue_2 "User.Yaxis" Yaxis)
      (Effects|Components|ParticleSystem|SetVectorParameter _returnvalue_2 "User.Zaxis" Zaxis))))

(fn FunctSpawnStMeshVR
  (params (AttachToComponent :type Scene%20Component%20Object%20Reference) (PortalLocation :type Vector) (MeshLocation :type Vector) (Color :type Linear%20Color%20Structure) (Size :type Float%20%28double-precision%29) (Xaxis :type Vector) (Yaxis :type Vector) (Zaxis :type Vector))
  (bind _returnvalue (Niagara|SpawnSystemAttached "/Game/Portals_VFXPack/VR/Particles/P_VR_SpawnStMesh.P_VR_SpawnStMesh" AttachToComponent "None" "0, 0, 0" "0, 0, 0" "KeepRelativeOffset" true))
  (Effects|Components|ParticleSystem|SetVectorParameter _returnvalue "User.EndLocation" PortalLocation)
  (Effects|Components|ParticleSystem|SetVectorParameter _returnvalue "User.StartLocation" MeshLocation)
  (Effects|Components|ParticleSystem|SetColorParameter _returnvalue "User.Color" Color)
  (Effects|Components|ParticleSystem|SetFloatParameter _returnvalue "User.Size" Size)
  (Effects|Components|ParticleSystem|SetVectorParameter _returnvalue "User.Xaxis" Xaxis)
  (Effects|Components|ParticleSystem|SetVectorParameter _returnvalue "User.Yaxis" Yaxis)
  (Effects|Components|ParticleSystem|SetVectorParameter _returnvalue "User.Zaxis" Zaxis))

(fn FunctSpawnSkMeshVR
  (params (AttachToComponent :type Scene%20Component%20Object%20Reference) (PortalLocation :type Vector) (MeshLocation :type Vector) (Color :type Linear%20Color%20Structure) (Size :type Float%20%28double-precision%29) (Xaxis :type Vector) (Yaxis :type Vector) (Zaxis :type Vector))
  (bind _returnvalue (Niagara|SpawnSystemAttached "/Game/Portals_VFXPack/VR/Particles/P_VR_SpawnSkMesh.P_VR_SpawnSkMesh" AttachToComponent "None" "0, 0, 0" "0, 0, 0" "KeepRelativeOffset" true))
  (Effects|Components|ParticleSystem|SetVectorParameter _returnvalue "User.EndLocation" PortalLocation)
  (Effects|Components|ParticleSystem|SetVectorParameter _returnvalue "User.StartLocation" MeshLocation)
  (Effects|Components|ParticleSystem|SetColorParameter _returnvalue "User.Color" Color)
  (Effects|Components|ParticleSystem|SetFloatParameter _returnvalue "User.Size" Size)
  (Effects|Components|ParticleSystem|SetVectorParameter _returnvalue "User.Xaxis" Xaxis)
  (Effects|Components|ParticleSystem|SetVectorParameter _returnvalue "User.Yaxis" Yaxis)
  (Effects|Components|ParticleSystem|SetVectorParameter _returnvalue "User.Zaxis" Zaxis))