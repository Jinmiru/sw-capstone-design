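; Manager actor that drives the two scene captures behind a linked pair of portals, so each portal's capture shows the view from the other.
; A FlipFlop on Tick alternates captures, so only one renders per frame.
; Each tick it then moves each capture to the opposite portal, remapping that portal's axes so the capture faces along its up vector.
; The low-poly portal pair is used only when Portal1 is invalid.
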(event EventTick
  (params (DeltaSeconds :type Float%20%28single-precision%29))
  (bind _scenecapture_portal2 (Variables|Default|GetSceneCapture_Portal2))
  (bind _portallowpoly2 (Variables|Default|GetPortalLowPoly2))
  (bind _portal2 (Variables|Default|GetPortal2))
  (bind _scenecapture_portal1 (Variables|Default|GetSceneCapture_Portal1))
  (bind _scenecapture_portal1_2 (Variables|Default|GetSceneCapture_Portal1))
  (bind _portallowpoly1 (Variables|Default|GetPortalLowPoly1))
  (bind _scenecapture_portal2_2 (Variables|Default|GetSceneCapture_Portal2))
  (bind _portal1 (Variables|Default|GetPortal1))
  (Utilities|FlowControl|Sequence
    (:then_0
      (Utilities|FlowControl|FlipFlop
        (:A
          (Rendering|SceneCapture|CaptureScene (Variables|Default|GetSceneCapture_Portal1) :!class /Script/Engine.SceneCaptureComponent2D))
        (:B
          (Rendering|SceneCapture|CaptureScene (Variables|Default|GetSceneCapture_Portal2) :!class /Script/Engine.SceneCaptureComponent2D))))
    (:then_1
      (Utilities|IsValid (Variables|Default|GetPortal1)
        (:Is%20Valid
          (Utilities|IsValid _portal2
            (:Is%20Valid
              (Utilities|FlowControl|Sequence
                (:then_0
                  (Transformation|SetWorldLocation _scenecapture_portal1 (Transformation|GetActorLocation _portal2) false true)
                  (Transformation|SetWorldRotation _scenecapture_portal1 (Math|Rotator|MakeRotationfromAxes (Transformation|GetActorUpVector _portal2) (* (Transformation|GetActorRightVector _portal2) -1.0) (Transformation|GetActorForwardVector _portal2)) false false))
                (:then_1
                  (Transformation|SetWorldLocation _scenecapture_portal2_2 (Transformation|GetActorLocation _portal1) false true)
                  (Transformation|SetWorldRotation _scenecapture_portal2_2 (Math|Rotator|MakeRotationfromAxes (Transformation|GetActorUpVector _portal1) (* (Transformation|GetActorRightVector _portal1) -1.0) (Transformation|GetActorForwardVector _portal1)) false false))))))
        (:Is%20Not%20Valid
          (Utilities|IsValid (Variables|Default|GetPortalLowPoly1)
            (:Is%20Valid
              (Utilities|IsValid _portallowpoly2
                (:Is%20Valid
                  (Utilities|FlowControl|Sequence
                    (:then_0
                      (Transformation|SetWorldLocation _scenecapture_portal1_2 (Transformation|GetActorLocation _portallowpoly2) false true)
                      (Transformation|SetWorldRotation _scenecapture_portal1_2 (Math|Rotator|MakeRotationfromAxes (Transformation|GetActorUpVector _portallowpoly2) (* (Transformation|GetActorRightVector _portallowpoly2) -1.0) (Transformation|GetActorForwardVector _portallowpoly2)) false false))
                    (:then_1
                      (Transformation|SetWorldLocation _scenecapture_portal2 (Transformation|GetActorLocation _portallowpoly1) false true)
                      (Transformation|SetWorldRotation _scenecapture_portal2 (Math|Rotator|MakeRotationfromAxes (Transformation|GetActorUpVector _portallowpoly1) (* (Transformation|GetActorRightVector _portallowpoly1) -1.0) (Transformation|GetActorForwardVector _portallowpoly1)) false false))))))))))))

(fn ConstructionScript)