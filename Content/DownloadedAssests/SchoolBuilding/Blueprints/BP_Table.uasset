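; Four-seat computer table prop that randomizes the placement of its monitors, keyboards, mice and chairs for a cluttered look.
; The construction script jitters them when the self-resetting RandomTransform toggle is set, then always rebuilds the cables.
; UpdateSplineWire snaps each spline's first point to its anchor component and adds spline meshes with a scaled wire material.
; Events re-randomize the layout, clearing and respawning wires, or toggle chair physics.
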(event Custom|ClearSplineWire
  (bind _output_get (Variables|Default|SetNewVar (Actor|GetComponentsByClass "/Script/Engine.SplineMeshComponent")))
  (for _array_element _output_get
    (Components|DestroyComponent _array_element)))

(event Custom|Update
  (bind _returnvalue (Math|Random|RandomFloatinRange 0.0 3.6e+02))
  (bind _returnvalue_2 (Math|Random|RandomPointinBoundingBox "0, 0, 0" "30.000000,30.000000,0.000000"))
  (bind _returnvalue_3 (Math|Random|RandomFloatinRange -75.0 -115.0))
  (bind _returnvalue_4 (Math|Random|RandomPointinBoundingBox "0, 0, 0" "10.000000,10.000000,0.000000"))
  (bind _returnvalue_5 (Math|Random|RandomPointinBoundingBox "0, 0, 0" "5.000000,5.000000,0.000000"))
  (bind _returnvalue_6 (Math|Random|RandomFloatinRange 75.0 115.0))
  (bind _returnvalue_7 (Math|Random|RandomFloatinRange -1e+01 1e+01))
  (bind _returnvalue_8 (Math|Random|RandomPointinBoundingBox "0, 0, 0" "5.000000,5.000000,0.000000"))
  (bind _returnvalue_9 (Math|Random|RandomFloatinRange 1.7e+02 1.9e+02))
  (bind _sm_monitor_plane3_staticmeshcomponent0 (Variables|Default|GetSM_Monitor_Plane3_StaticMeshComponent0))
  (bind _sm_monitor_plane2_staticmeshcomponent0 (Variables|Default|GetSM_Monitor_Plane2_StaticMeshComponent0))
  (bind _sm_keyborad_mouse2_staticmeshcomponent0 (Variables|Default|GetSM_Keyborad_Mouse2_StaticMeshComponent0))
  (bind _sm_keyborad_keyborad_staticmeshcomponent0 (Variables|Default|GetSM_Keyborad_KeyBorad_StaticMeshComponent0))
  (bind _sm_keyborad_mouse_staticmeshcomponent0 (Variables|Default|GetSM_Keyborad_Mouse_StaticMeshComponent0))
  (bind _sm_keyborad_keyborad2_staticmeshcomponent0 (Variables|Default|GetSM_Keyborad_KeyBorad2_StaticMeshComponent0))
  (bind _sm_keyborad_keyborad4_staticmeshcomponent0 (Variables|Default|GetSM_Keyborad_KeyBorad4_StaticMeshComponent0))
  (bind _sm_keyborad_keyborad3_staticmeshcomponent0 (Variables|Default|GetSM_Keyborad_KeyBorad3_StaticMeshComponent0))
  (bind _sm_keyborad_mouse3_staticmeshcomponent0 (Variables|Default|GetSM_Keyborad_Mouse3_StaticMeshComponent0))
  (bind _sm_keyborad_mouse4_staticmeshcomponent0 (Variables|Default|GetSM_Keyborad_Mouse4_StaticMeshComponent0))
  (bind _sm_chair_circle_8_staticmeshcomponent0 (Variables|Default|GetSM_chair_Circle_8_StaticMeshComponent0))
  (bind _sm_chair_circle_9_staticmeshcomponent0 (Variables|Default|GetSM_chair_Circle_9_StaticMeshComponent0))
  (bind _sm_chair_circle_10_staticmeshcomponent0 (Variables|Default|GetSM_chair_Circle_10_StaticMeshComponent0))
  (bind _sm_chair_circle_007_staticmeshcomponent0 (Variables|Default|GetSM_chair_Circle_007_StaticMeshComponent0))
  (bind _sm_monitor_plane4_staticmeshcomponent0 (Variables|Default|GetSM_Monitor_Plane4_StaticMeshComponent0))
  (bind _returnvalue_10 (Math|Rotator|MakeRotator 0.0 0.0 _returnvalue_3))
  (bind _returnvalue_11 (Math|Rotator|MakeRotator 0.0 0.0 _returnvalue))
  (bind _returnvalue_12 (Math|Rotator|MakeRotator 0.0 0.0 _returnvalue_6))
  (bind _returnvalue_13 (Math|Rotator|MakeRotator 0.0 0.0 _returnvalue_7))
  (bind _returnvalue_14 (Math|Rotator|MakeRotator 0.0 0.0 _returnvalue_9))
  (Utilities|FlowControl|Sequence
    (:then_0
      (CallFunction|ClearSplineWire))
    (:then_1
      (Transformation|AddWorldOffset (Variables|Default|GetSM_Monitor_Plane_StaticMeshComponent0) _returnvalue_4 false false)
      (Transformation|AddWorldOffset _sm_monitor_plane3_staticmeshcomponent0 _returnvalue_4 false false)
      (Transformation|AddWorldOffset _sm_monitor_plane2_staticmeshcomponent0 _returnvalue_4 false false)
      (Transformation|AddWorldOffset _sm_monitor_plane4_staticmeshcomponent0 _returnvalue_4 false false)
      (Transformation|SetRelativeRotation _sm_monitor_plane3_staticmeshcomponent0 _returnvalue_10 false false)
      (Transformation|SetRelativeRotation _sm_monitor_plane3_staticmeshcomponent0 _returnvalue_12 false false)
      (Transformation|SetRelativeRotation _sm_monitor_plane2_staticmeshcomponent0 _returnvalue_10 false false)
      (Transformation|SetRelativeRotation _sm_monitor_plane4_staticmeshcomponent0 _returnvalue_12 false false)
      (Transformation|AddWorldOffset _sm_keyborad_mouse2_staticmeshcomponent0 _returnvalue_5 false false)
      (Transformation|AddWorldOffset _sm_keyborad_keyborad_staticmeshcomponent0 _returnvalue_5 false false)
      (Transformation|AddWorldOffset _sm_keyborad_mouse_staticmeshcomponent0 _returnvalue_5 false false)
      (Transformation|AddWorldOffset _sm_keyborad_keyborad2_staticmeshcomponent0 _returnvalue_5 false false)
      (Transformation|SetRelativeRotation _sm_keyborad_mouse2_staticmeshcomponent0 _returnvalue_13 false false)
      (Transformation|SetRelativeRotation _sm_keyborad_keyborad_staticmeshcomponent0 _returnvalue_13 false false)
      (Transformation|SetRelativeRotation _sm_keyborad_mouse_staticmeshcomponent0 _returnvalue_13 false false)
      (Transformation|SetRelativeRotation _sm_keyborad_keyborad2_staticmeshcomponent0 _returnvalue_13 false false)
      (Transformation|AddWorldOffset _sm_keyborad_keyborad4_staticmeshcomponent0 _returnvalue_8 false false)
      (Transformation|AddWorldOffset _sm_keyborad_keyborad3_staticmeshcomponent0 _returnvalue_8 false false)
      (Transformation|AddWorldOffset _sm_keyborad_mouse3_staticmeshcomponent0 _returnvalue_8 false false)
      (Transformation|AddWorldOffset _sm_keyborad_mouse4_staticmeshcomponent0 _returnvalue_8 false false)
      (Transformation|SetRelativeRotation _sm_keyborad_keyborad4_staticmeshcomponent0 _returnvalue_14 false false)
      (Transformation|SetRelativeRotation _sm_keyborad_keyborad3_staticmeshcomponent0 _returnvalue_14 false false)
      (Transformation|SetRelativeRotation _sm_keyborad_mouse3_staticmeshcomponent0 _returnvalue_14 false false)
      (Transformation|SetRelativeRotation _sm_keyborad_mouse4_staticmeshcomponent0 _returnvalue_14 false false)
      (Transformation|AddWorldOffset _sm_chair_circle_8_staticmeshcomponent0 _returnvalue_2 false false)
      (Transformation|AddWorldOffset _sm_chair_circle_9_staticmeshcomponent0 _returnvalue_2 false false)
      (Transformation|AddWorldOffset _sm_chair_circle_10_staticmeshcomponent0 _returnvalue_2 false false)
      (Transformation|AddWorldOffset _sm_chair_circle_007_staticmeshcomponent0 _returnvalue_2 false false)
      (Transformation|SetRelativeRotation _sm_chair_circle_8_staticmeshcomponent0 _returnvalue_11 false false)
      (Transformation|SetRelativeRotation _sm_chair_circle_9_staticmeshcomponent0 _returnvalue_11 false false)
      (Transformation|SetRelativeRotation _sm_chair_circle_10_staticmeshcomponent0 _returnvalue_11 false false)
      (Transformation|SetRelativeRotation _sm_chair_circle_007_staticmeshcomponent0 _returnvalue_11 false false)
      (CallFunction|SpawnSplineWire))))

(event Custom|SetChairPhysicSim
  (params (NewParam :type Boolean))
  (Physics|SetSimulatePhysics (Variables|Default|GetSM_chair_Circle_007_StaticMeshComponent0) NewParam))

(event Custom|SpawnSplineWire
  (CallFunction|UpdateSplineWire (Variables|Default|Getm1w) -0.8 (Transformation|GetWorldLocation (Variables|Default|Getm1)))
  (CallFunction|UpdateSplineWire (Variables|Default|Getk1w) -0.8 (Transformation|GetWorldLocation (Variables|Default|Getk1)))
  (CallFunction|UpdateSplineWire (Variables|Default|Getm2w) -0.8 (Transformation|GetWorldLocation (Variables|Default|Getm2)))
  (CallFunction|UpdateSplineWire (Variables|Default|Getk2w) -0.8 (Transformation|GetWorldLocation (Variables|Default|Getk2)))
  (CallFunction|UpdateSplineWire (Variables|Default|Getm3w) -0.8 (Transformation|GetWorldLocation (Variables|Default|Getm3)))
  (CallFunction|UpdateSplineWire (Variables|Default|Getk3w) -0.8 (Transformation|GetWorldLocation (Variables|Default|Getk3)))
  (CallFunction|UpdateSplineWire (Variables|Default|Getm4w) -0.8 (Transformation|GetWorldLocation (Variables|Default|Getm4)))
  (CallFunction|UpdateSplineWire (Variables|Default|Getk4w) -0.8 (Transformation|GetWorldLocation (Variables|Default|Getk4)))
  (CallFunction|UpdateSplineWire (Variables|Default|Getwoa1) -1.4 (Transformation|GetWorldLocation (Variables|Default|Getoa1)))
  (CallFunction|UpdateSplineWire (Variables|Default|Getwoa2) -1.4 (Transformation|GetWorldLocation (Variables|Default|Getoa2)))
  (CallFunction|UpdateSplineWire (Variables|Default|Getwoa3) -1.4 (Transformation|GetWorldLocation (Variables|Default|Getoa3)))
  (CallFunction|UpdateSplineWire (Variables|Default|Getwoa4) -1.4 (Transformation|GetWorldLocation (Variables|Default|Getoa4)))
  (CallFunction|UpdateSplineWire (Variables|Default|Getwob2) -1.3 (Transformation|GetWorldLocation (Variables|Default|Getob1)))
  (CallFunction|UpdateSplineWire (Variables|Default|Getwob1) -1.3 (Transformation|GetWorldLocation (Variables|Default|Getob2)))
  (CallFunction|UpdateSplineWire (Variables|Default|Getwob3) -1.3 (Transformation|GetWorldLocation (Variables|Default|Getob3)))
  (CallFunction|UpdateSplineWire (Variables|Default|Getwob4) -1.3 (Transformation|GetWorldLocation (Variables|Default|Getob4))))

(event EventBeginPlay)

(event Collision|EventActorBeginOverlap
  (params (OtherActor :type Actor%20Object%20Reference)))

(event EventTick
  (params (DeltaSeconds :type Float%20%28single-precision%29)))

(fn ConstructionScript
  (bind _returnvalue (Math|Random|RandomFloatinRange 0.0 3.6e+02))
  (bind _returnvalue_2 (Math|Random|RandomPointinBoundingBox "0, 0, 0" "30.000000,30.000000,0.000000"))
  (bind _returnvalue_3 (Math|Random|RandomFloatinRange -75.0 -115.0))
  (bind _returnvalue_4 (Math|Random|RandomPointinBoundingBox "0, 0, 0" "20.000000,20.000000,0.000000"))
  (bind _returnvalue_5 (Math|Random|RandomPointinBoundingBox "0, 0, 0" "10.000000,10.000000,0.000000"))
  (bind _returnvalue_6 (Math|Random|RandomFloatinRange 75.0 115.0))
  (bind _returnvalue_7 (Math|Random|RandomFloatinRange -1e+01 1e+01))
  (bind _returnvalue_8 (Math|Random|RandomPointinBoundingBox "0, 0, 0" "10.000000,10.000000,0.000000"))
  (bind _returnvalue_9 (Math|Random|RandomFloatinRange 1.7e+02 1.9e+02))
  (bind _sm_monitor_plane3_staticmeshcomponent0 (Variables|Default|GetSM_Monitor_Plane3_StaticMeshComponent0))
  (bind _sm_monitor_plane2_staticmeshcomponent0 (Variables|Default|GetSM_Monitor_Plane2_StaticMeshComponent0))
  (bind _sm_keyborad_mouse2_staticmeshcomponent0 (Variables|Default|GetSM_Keyborad_Mouse2_StaticMeshComponent0))
  (bind _sm_keyborad_keyborad_staticmeshcomponent0 (Variables|Default|GetSM_Keyborad_KeyBorad_StaticMeshComponent0))
  (bind _sm_keyborad_mouse_staticmeshcomponent0 (Variables|Default|GetSM_Keyborad_Mouse_StaticMeshComponent0))
  (bind _sm_keyborad_keyborad2_staticmeshcomponent0 (Variables|Default|GetSM_Keyborad_KeyBorad2_StaticMeshComponent0))
  (bind _sm_keyborad_keyborad4_staticmeshcomponent0 (Variables|Default|GetSM_Keyborad_KeyBorad4_StaticMeshComponent0))
  (bind _sm_keyborad_keyborad3_staticmeshcomponent0 (Variables|Default|GetSM_Keyborad_KeyBorad3_StaticMeshComponent0))
  (bind _sm_keyborad_mouse3_staticmeshcomponent0 (Variables|Default|GetSM_Keyborad_Mouse3_StaticMeshComponent0))
  (bind _sm_keyborad_mouse4_staticmeshcomponent0 (Variables|Default|GetSM_Keyborad_Mouse4_StaticMeshComponent0))
  (bind _sm_chair_circle_8_staticmeshcomponent0 (Variables|Default|GetSM_chair_Circle_8_StaticMeshComponent0))
  (bind _sm_chair_circle_9_staticmeshcomponent0 (Variables|Default|GetSM_chair_Circle_9_StaticMeshComponent0))
  (bind _sm_chair_circle_10_staticmeshcomponent0 (Variables|Default|GetSM_chair_Circle_10_StaticMeshComponent0))
  (bind _sm_chair_circle_007_staticmeshcomponent0 (Variables|Default|GetSM_chair_Circle_007_StaticMeshComponent0))
  (bind _sm_monitor_plane4_staticmeshcomponent0 (Variables|Default|GetSM_Monitor_Plane4_StaticMeshComponent0))
  (bind _returnvalue_10 (Math|Rotator|MakeRotator 0.0 0.0 _returnvalue_3))
  (bind _returnvalue_11 (Math|Rotator|MakeRotator 0.0 0.0 _returnvalue))
  (bind _returnvalue_12 (Math|Rotator|MakeRotator 0.0 0.0 _returnvalue_6))
  (bind _returnvalue_13 (Math|Rotator|MakeRotator 0.0 0.0 _returnvalue_7))
  (bind _returnvalue_14 (Math|Rotator|MakeRotator 0.0 0.0 _returnvalue_9))
  (Utilities|FlowControl|Sequence
    (:then_0
      (if (Variables|Default|GetRandomTransform)
        (Variables|Default|SetRandomTransform false)
        (Transformation|AddWorldOffset (Variables|Default|GetSM_Monitor_Plane_StaticMeshComponent0) _returnvalue_4 false false)
        (Transformation|AddWorldOffset _sm_monitor_plane3_staticmeshcomponent0 _returnvalue_4 false false)
        (Transformation|AddWorldOffset _sm_monitor_plane2_staticmeshcomponent0 _returnvalue_4 false false)
        (Transformation|AddWorldOffset _sm_monitor_plane4_staticmeshcomponent0 _returnvalue_4 false false)
        (Transformation|SetRelativeRotation _sm_monitor_plane3_staticmeshcomponent0 _returnvalue_10 false false)
        (Transformation|SetRelativeRotation _sm_monitor_plane3_staticmeshcomponent0 _returnvalue_12 false false)
        (Transformation|SetRelativeRotation _sm_monitor_plane2_staticmeshcomponent0 _returnvalue_10 false false)
        (Transformation|SetRelativeRotation _sm_monitor_plane4_staticmeshcomponent0 _returnvalue_12 false false)
        (Transformation|AddWorldOffset _sm_keyborad_mouse2_staticmeshcomponent0 _returnvalue_5 false false)
        (Transformation|AddWorldOffset _sm_keyborad_keyborad_staticmeshcomponent0 _returnvalue_5 false false)
        (Transformation|AddWorldOffset _sm_keyborad_mouse_staticmeshcomponent0 _returnvalue_5 false false)
        (Transformation|AddWorldOffset _sm_keyborad_keyborad2_staticmeshcomponent0 _returnvalue_5 false false)
        (Transformation|SetRelativeRotation _sm_keyborad_mouse2_staticmeshcomponent0 _returnvalue_13 false false)
        (Transformation|SetRelativeRotation _sm_keyborad_keyborad_staticmeshcomponent0 _returnvalue_13 false false)
        (Transformation|SetRelativeRotation _sm_keyborad_mouse_staticmeshcomponent0 _returnvalue_13 false false)
        (Transformation|SetRelativeRotation _sm_keyborad_keyborad2_staticmeshcomponent0 _returnvalue_13 false false)
        (Transformation|AddWorldOffset _sm_keyborad_keyborad4_staticmeshcomponent0 _returnvalue_8 false false)
        (Transformation|AddWorldOffset _sm_keyborad_keyborad3_staticmeshcomponent0 _returnvalue_8 false false)
        (Transformation|AddWorldOffset _sm_keyborad_mouse3_staticmeshcomponent0 _returnvalue_8 false false)
        (Transformation|AddWorldOffset _sm_keyborad_mouse4_staticmeshcomponent0 _returnvalue_8 false false)
        (Transformation|SetRelativeRotation _sm_keyborad_keyborad4_staticmeshcomponent0 _returnvalue_14 false false)
        (Transformation|SetRelativeRotation _sm_keyborad_keyborad3_staticmeshcomponent0 _returnvalue_14 false false)
        (Transformation|SetRelativeRotation _sm_keyborad_mouse3_staticmeshcomponent0 _returnvalue_14 false false)
        (Transformation|SetRelativeRotation _sm_keyborad_mouse4_staticmeshcomponent0 _returnvalue_14 false false)
        (Transformation|AddWorldOffset _sm_chair_circle_8_staticmeshcomponent0 _returnvalue_2 false false)
        (Transformation|AddWorldOffset _sm_chair_circle_9_staticmeshcomponent0 _returnvalue_2 false false)
        (Transformation|AddWorldOffset _sm_chair_circle_10_staticmeshcomponent0 _returnvalue_2 false false)
        (Transformation|AddWorldOffset _sm_chair_circle_007_staticmeshcomponent0 _returnvalue_2 false false)
        (Transformation|SetRelativeRotation _sm_chair_circle_8_staticmeshcomponent0 _returnvalue_11 false false)
        (Transformation|SetRelativeRotation _sm_chair_circle_9_staticmeshcomponent0 _returnvalue_11 false false)
        (Transformation|SetRelativeRotation _sm_chair_circle_10_staticmeshcomponent0 _returnvalue_11 false false)
        (Transformation|SetRelativeRotation _sm_chair_circle_007_staticmeshcomponent0 _returnvalue_11 false false)))
    (:then_1
      (CallFunction|UpdateSplineWire (Variables|Default|Getm1w) -0.8 (Transformation|GetWorldLocation (Variables|Default|Getm1)))
      (CallFunction|UpdateSplineWire (Variables|Default|Getk1w) -0.8 (Transformation|GetWorldLocation (Variables|Default|Getk1)))
      (CallFunction|UpdateSplineWire (Variables|Default|Getm2w) -0.8 (Transformation|GetWorldLocation (Variables|Default|Getm2)))
      (CallFunction|UpdateSplineWire (Variables|Default|Getk2w) -0.8 (Transformation|GetWorldLocation (Variables|Default|Getk2)))
      (CallFunction|UpdateSplineWire (Variables|Default|Getm3w) -0.8 (Transformation|GetWorldLocation (Variables|Default|Getm3)))
      (CallFunction|UpdateSplineWire (Variables|Default|Getk3w) -0.8 (Transformation|GetWorldLocation (Variables|Default|Getk3)))
      (CallFunction|UpdateSplineWire (Variables|Default|Getm4w) -0.8 (Transformation|GetWorldLocation (Variables|Default|Getm4)))
      (CallFunction|UpdateSplineWire (Variables|Default|Getk4w) -0.8 (Transformation|GetWorldLocation (Variables|Default|Getk4)))
      (CallFunction|UpdateSplineWire (Variables|Default|Getwoa1) -1.4 (Transformation|GetWorldLocation (Variables|Default|Getoa1)))
      (CallFunction|UpdateSplineWire (Variables|Default|Getwoa2) -1.4 (Transformation|GetWorldLocation (Variables|Default|Getoa2)))
      (CallFunction|UpdateSplineWire (Variables|Default|Getwoa3) -1.4 (Transformation|GetWorldLocation (Variables|Default|Getoa3)))
      (CallFunction|UpdateSplineWire (Variables|Default|Getwoa4) -1.4 (Transformation|GetWorldLocation (Variables|Default|Getoa4)))
      (CallFunction|UpdateSplineWire (Variables|Default|Getwob2) -1.3 (Transformation|GetWorldLocation (Variables|Default|Getob1)))
      (CallFunction|UpdateSplineWire (Variables|Default|Getwob1) -1.3 (Transformation|GetWorldLocation (Variables|Default|Getob2)))
      (CallFunction|UpdateSplineWire (Variables|Default|Getwob3) -1.3 (Transformation|GetWorldLocation (Variables|Default|Getob3)))
      (CallFunction|UpdateSplineWire (Variables|Default|Getwob4) -1.3 (Transformation|GetWorldLocation (Variables|Default|Getob4))))))

(fn UpdateSplineWire
  (params (InputPin :type Spline%20Component%20Object%20Reference) (Scale :type Float%20%28single-precision%29) (FirstPointLocation :type Vector%20%28by%20ref%29))
  (Spline|SetLocationatSplinePoint InputPin 0 FirstPointLocation "World" true)
  (for _index (range 0 (- (Spline|GetNumberOfSplinePoints InputPin) 2))
    (bind _returnvalue (AddComponent|AddSplineMeshComponent false))
    (bind _returnvalue_2 (Rendering|Material|CreateDynamicMaterialInstance _returnvalue 0 "/Game/DownloadedAssests/SchoolBuilding/Material/MI_Wire.MI_Wire" "None" :!class /Script/Engine.PrimitiveComponent))
    (Rendering|Material|SetScalarParameterValue _returnvalue_2 "Scale" Scale :!class /Script/Engine.MaterialInstanceDynamic)
    (Transformation|AttachComponentToComponent _returnvalue InputPin "None" "KeepRelative" "KeepRelative" "KeepRelative" true)
    (SplineMesh|SetStartandEnd _returnvalue (.Location (Spline|GetLocationandTangentatSplinePoint InputPin _index "Local")) (.Tangent (Spline|GetLocationandTangentatSplinePoint InputPin _index "Local")) (.Location (Spline|GetLocationandTangentatSplinePoint InputPin (+ _index 1) "Local")) (.Tangent (Spline|GetLocationandTangentatSplinePoint InputPin (+ _index 1) "Local")) true :!class /Script/Engine.SplineMeshComponent)))