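; Stair door actor for School Building 5 that randomizes how open its two door leaves appear in the level.
; The construction script sets a random yaw on two arrow components, mirrored in sign for each side.
; Each side independently picks either a wide-open angle around a right angle or a nearly closed one.
; The event graph holds only disabled stubs, so there is no runtime behavior.
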(event EventBeginPlay)

(event Collision|EventActorBeginOverlap
  (params (OtherActor :type Actor%20Object%20Reference)))

(event EventTick
  (params (DeltaSeconds :type Float%20%28single-precision%29)))

(fn ConstructionScript
  (bind _returnvalue (Math|Random|RandomBool))
  (Transformation|SetRelativeRotation (Variables|Default|GetArrow) (Math|Rotator|MakeRotator 0.0 0.0 (Math|Float|SelectFloat (Math|Random|RandomFloatinRange 9e+01 1.1e+02) (Math|Random|RandomFloatinRange 0.0 1e+01) _returnvalue)) false false)
  (Transformation|SetRelativeRotation (Variables|Default|GetArrow1) (Math|Rotator|MakeRotator 0.0 0.0 (Math|Float|SelectFloat (Math|Random|RandomFloatinRange -9e+01 -1.1e+02) (Math|Random|RandomFloatinRange 0.0 -1e+01) _returnvalue)) false false))