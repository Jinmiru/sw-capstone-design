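; BP_Building5_Room is a school building room prefab that varies the openness of its doors and windows on each construction.
; The construction script rolls random yaw angles for the room, toilet and outer doors, and random Y offsets to slide two windows.
; Coin flips can leave the room door and either window at their zero position, while the other doors always get a random angle.
; It has no active runtime logic.
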(event EventBeginPlay)

(event Collision|EventActorBeginOverlap
  (params (OtherActor :type Actor%20Object%20Reference)))

(event EventTick
  (params (DeltaSeconds :type Float%20%28single-precision%29)))

(fn ConstructionScript
  (bind _returnvalue (Math|Random|RandomFloatinRange 0.0 -9e+01))
  (bind _returnvalue_2 (Math|Random|RandomFloatinRange 0.0 9e+01))
  (bind _returnvalue_3 (Math|Random|RandomBool))
  (Variables|Default|SetRotate_Door (Math|Float|SelectFloat 0.0 _returnvalue (Math|Random|RandomBool)))
  (Variables|Default|SetRotate_ToiletDoorL _returnvalue)
  (Variables|Default|SetRotate_ToiletDoorR _returnvalue_2)
  (Variables|Default|SetRotate_DoorOut _returnvalue_2)
  (Variables|Default|SetOffset_WindowL (Math|Float|SelectFloat (Math|Random|RandomFloatinRange 0.0 -6e+01) 0.0 _returnvalue_3))
  (Variables|Default|SetOffset_WindowLR (Math|Float|SelectFloat (Math|Random|RandomFloatinRange 0.0 6e+01) 0.0 _returnvalue_3))
  (Transformation|SetRelativeLocation (Variables|Default|Getw1) (Math|Vector|MakeVector 0.0 (Variables|Default|GetOffset_WindowL) 0.0) false false)
  (Transformation|SetRelativeLocation (Variables|Default|Getw3) (Math|Vector|MakeVector 0.0 (Variables|Default|GetOffset_WindowLR) 0.0) false false)
  (Transformation|SetRelativeRotation (Variables|Default|GetDoor_room) (Math|Rotator|MakeRotator 0.0 0.0 (Variables|Default|GetRotate_Door)) false false)
  (Transformation|SetRelativeRotation (Variables|Default|GetToilet_l) (Math|Rotator|MakeRotator 0.0 0.0 (Variables|Default|GetRotate_ToiletDoorL)) false false)
  (Transformation|SetRelativeRotation (Variables|Default|GetToilet_r) (Math|Rotator|MakeRotator 0.0 0.0 (Variables|Default|GetRotate_ToiletDoorR)) false false)
  (Transformation|SetRelativeRotation (Variables|Default|Getdoor_out) (Math|Rotator|MakeRotator 0.0 0.0 (Variables|Default|GetRotate_DoorOut)) false false))