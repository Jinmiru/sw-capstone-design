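; BP_Building5 is a procedural school building that assembles itself from a room count (Room) and a floor count (Layer).
; The ReSpawn toggle in the construction script, or the SpawnStart event, calls SpawnBase; BeginPlay does nothing.
; Spawn_base loops along Y and up Z, adding mesh instances for ends, corridors, floors and top pieces, plus child actors.
; Negative Y scale mirrors the far end, and a FlipFlop alternates floor-piece patterns.
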(event Custom|SpawnStart
  (Utilities|SpawnBase))

(event EventBeginPlay)

(fn ConstructionScript
  (if (Variables|Default|GetReSpawn)
    (Variables|Default|SetReSpawn false)
    (Utilities|SpawnBase)))