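; Traffic light actor that cycles vehicle or pedestrian signal lamps, with LightType choosing the variant.
; The construction script swaps in the pedestrian light mesh for both pedestrian types.
; On BeginPlay a timeline plays, with phase-shift types starting at an offset position so lights can run out of step.
; Each update writes the timeline's curves to red, yellow, green and pedestrian scalar parameters on the mesh materials.
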(event EventBeginPlay
  (bind _sm_trafficlight (Variables|Default|GetSM_TrafficLight))
  (switch Utilities|FlowControl|Switch|SwitchonE_TrafficLights (Variables|Default|GetLight%20Type)
    (:NewEnumerator0
      (bind (_direction _traffic_lights _pedestrian) (Timeline|Traffic%20Light Play)
        (:Update
          (Rendering|Material|SetScalarParameterValueonMaterials _sm_trafficlight "Red" (.X (Math|Vector|BreakVector _traffic_lights)))
          (Rendering|Material|SetScalarParameterValueonMaterials _sm_trafficlight "Yellow" (.Z (Math|Vector|BreakVector _traffic_lights)))
          (Rendering|Material|SetScalarParameterValueonMaterials _sm_trafficlight "Green" (.Y (Math|Vector|BreakVector _traffic_lights)))
          (Rendering|Material|SetScalarParameterValueonMaterials _sm_trafficlight "RedP" (.X (Math|Vector|BreakVector _pedestrian)))
          (Rendering|Material|SetScalarParameterValueonMaterials _sm_trafficlight "GreenP" (.Y (Math|Vector|BreakVector _pedestrian))))))
    (:NewEnumerator1
      (Components|Timeline|SetPlaybackPosition (Variables|Default|GetTraffic%20Light) 25.0 false true :!label _label)
      (Timeline|Traffic%20Light Play))
    (:NewEnumerator2
      (Timeline|Traffic%20Light Play))
    (:NewEnumerator3
      (goto _label))))

(event Collision|EventActorBeginOverlap
  (params (OtherActor :type Actor%20Object%20Reference)))

(event EventTick
  (params (DeltaSeconds :type Float%20%28single-precision%29)))

(fn ConstructionScript
  (switch Utilities|FlowControl|Switch|SwitchonE_TrafficLights (Variables|Default|GetLight%20Type)
    (:NewEnumerator2
      _)
    (:NewEnumerator3
      _))
  (Components|StaticMesh|SetStaticMesh (Variables|Default|GetSM_TrafficLight) "/Game/DownloadedAssests/ModernCityBundle/Meshes/StreetElements/SM_PedestrianLight.SM_PedestrianLight"))