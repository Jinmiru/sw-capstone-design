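; Street light actor that switches its spotlight and emissive lamp material on or off according to the third-person character's night flag.
; Every Tick it reapplies the configurable spotlight settings and reads IsNight from the first BP_ThirdPersonCharacter found through GetAllActorsOfClass.
; At night it applies glow, tint and either temperature or color.
; By day it zeroes glow and intensity and toggles spotlight visibility each frame.
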(event EventBeginPlay)

(event Collision|EventActorBeginOverlap
  (params (OtherActor :type Actor%20Object%20Reference)))

(event EventTick
  (params (DeltaSeconds :type Float%20%28single-precision%29))
  (bind _spotlight (Variables|Default|GetSpotLight))
  (bind _spotlight_2 (Variables|Default|GetSpotLight))
  (bind _spotlight_3 (Variables|Default|GetSpotLight))
  (bind _sm_street_light (Variables|Default|GetSM_Street_Light))
  (Transformation|SetMobility _spotlight (Variables|Default|GetLight%20Mobility))
  (Rendering|Components|Light|SetIntensity _spotlight (Variables|Default|GetLight%20Intensity))
  (Rendering|Lighting|SetAttenuationRadius _spotlight (Variables|Default|GetAttenuation%20Radius))
  (Rendering|Lighting|SetInnerConeAngle _spotlight (Variables|Default|GetInner%20Cone%20Angle))
  (Rendering|Lighting|SetOuterConeAngle _spotlight (Variables|Default|GetOuter%20Cone%20Angle))
  (Rendering|Components|Light|SetCastShadows _spotlight (Variables|Default|GetCast%20Shadows))
  (bind _outactors (Actor|GetAllActorsOfClass "/Game/ThirdPerson/Blueprints/BP_ThirdPersonCharacter.BP_ThirdPersonCharacter_C"))
  (bind _asbp_third_person_character (Utilities|Casting|CastToBP_ThirdPersonCharacter (Utilities|Array|Get(acopy) _outactors)))
  (bind _output_get (Variables|Default|SetLightON (Variables|/Script/MyProject.MyProjectCharacter|GetisNight _asbp_third_person_character)))
  (if _output_get
    (Rendering|Material|SetScalarParameterValueonMaterials _sm_street_light "LightIntensity" (Variables|Default|GetEmissive%20Intensity))
    (Rendering|Material|SetVectorParameterValueonMaterials _sm_street_light "Light Color" (Math|Conversions|ToVector(LinearColor) (Variables|Default|GetEmissive%20Tint)))
    (Class|LightComponent|SetIndirectLightingIntensity (Variables|Default|GetSpotLight) (Variables|Default|GetIndirect%20Lighting%20Intensity))
    (if (Variables|Default|GetUse%20Temperature)
      (Class|LightComponent|SetTemperature _spotlight_2 (Variables|Default|GetTemperature))
      (else
        (Rendering|Components|Light|SetLightColor _spotlight_2 (Variables|Default|GetLight%20Color) true)))
    (else
      (Rendering|Material|SetScalarParameterValueonMaterials (Variables|Default|GetSM_Street_Light) "LightIntensity" 0.0)
      (Rendering|ToggleVisibility _spotlight_3 false)
      (Rendering|Components|Light|SetIntensity _spotlight_3 0.0)
      (Class|LightComponent|SetIndirectLightingIntensity _spotlight_3 0.0))))

(fn ConstructionScript)