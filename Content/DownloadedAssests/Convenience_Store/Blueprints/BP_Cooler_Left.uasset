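; BP_Cooler_Left is a modular left-side cooler prop for a convenience store environment, configured per instance in the editor.
; Its construction script uses type variables to index arrays, setting the cooler body mesh and wallpaper material plus left and right door and shelf meshes.
; The wall type also decides whether the trim mesh comes from the corner or standard array.
; It has no active runtime logic.
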(event EventBeginPlay)

(event Collision|EventActorBeginOverlap
  (params (OtherActor :type Actor%20Object%20Reference)))

(event EventTick
  (params (DeltaSeconds :type Float%20%28single-precision%29)))

(fn ConstructionScript
  (bind _wall_type (Variables|Customization|GetWall_Type))
  (bind _returnvalue (Math|Conversions|ToInteger(Byte) _wall_type))
  (Rendering|Material|SetMaterial (Variables|Default|GetCooler) 0 (Utilities|Array|Get(acopy) (LocalVariables|GetWall_Materials) (Math|Conversions|ToInteger(Byte) (Variables|Customization|GetWallpaper_Type))))
  (Components|StaticMesh|SetStaticMesh (Variables|Default|GetCooler) (Utilities|Array|Get(acopy) (LocalVariables|GetCooler_Meshes) _returnvalue))
  (LocalVariables|SetCorner_Choice (== _returnvalue 1))
  (Components|StaticMesh|SetStaticMesh (Variables|Default|GetDoor_Left) (Utilities|Array|Get(acopy) (LocalVariables|GetDoor_Meshes) (Math|Conversions|ToInteger(Byte) (Variables|Customization|GetLeft_Door_Type))))
  (Components|StaticMesh|SetStaticMesh (Variables|Default|GetDoor_Right) (Utilities|Array|Get(acopy) (LocalVariables|GetDoor_Meshes) (Math|Conversions|ToInteger(Byte) (Variables|Customization|GetRight_Door_Type))))
  (Components|StaticMesh|SetStaticMesh (Variables|Default|GetShelf_Left) (Utilities|Array|Get(acopy) (LocalVariables|GetShelf_Meshes) (Math|Conversions|ToInteger(Byte) (Variables|Customization|GetShelf_Left_Type))))
  (Components|StaticMesh|SetStaticMesh (Variables|Default|GetShelf_Right) (Utilities|Array|Get(acopy) (LocalVariables|GetShelf_Meshes) (Math|Conversions|ToInteger(Byte) (Variables|Customization|GetShelf_Right_Type))))
  (if (LocalVariables|GetCorner_Choice)
    (Components|StaticMesh|SetStaticMesh (Variables|Default|GetWall_Trim) (Utilities|Array|Get(acopy) (LocalVariables|GetTrim_Corner_Meshes) (Math|Conversions|ToInteger(Byte) (Variables|Customization|GetWall_Trim_Type))))
    (else
      (Components|StaticMesh|SetStaticMesh (Variables|Default|GetWall_Trim) (Utilities|Array|Get(acopy) (LocalVariables|GetTrim_Meshes) (Math|Conversions|ToInteger(Byte) (Variables|Customization|GetWall_Trim_Type)))))))