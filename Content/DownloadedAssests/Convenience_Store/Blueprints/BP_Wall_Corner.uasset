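; BP_Wall_Corner is a modular wall corner piece for the convenience store environment, configured by wall, trim and wallpaper type.
; Its construction script sets the corner mesh and wallpaper material from arrays indexed by those types.
; The trim mesh comes from either an inside or regular array, depending on whether the wall type is the one at index 1.
; The event graph holds no active logic.
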(event EventBeginPlay)

(event Collision|EventActorBeginOverlap
  (params (OtherActor :type Actor%20Object%20Reference)))

(event EventTick
  (params (DeltaSeconds :type Float%20%28single-precision%29)))

(fn ConstructionScript
  (bind _wall_type (Variables|Customization|GetWall_Type))
  (bind _returnvalue (Math|Conversions|ToInteger(Byte) _wall_type))
  (Components|StaticMesh|SetStaticMesh (Variables|Default|GetWall_Corners) (Utilities|Array|Get(acopy) (LocalVariables|GetWall_Corner_Meshes) _returnvalue))
  (LocalVariables|SetWall_Inside_Choice (== _returnvalue 1))
  (if (LocalVariables|GetWall_Inside_Choice)
    (Components|StaticMesh|SetStaticMesh (Variables|Default|GetTrims) (Utilities|Array|Get(acopy) (LocalVariables|GetTrim_Meshes_Inside) (Math|Conversions|ToInteger(Byte) (Variables|Customization|GetTrim_Type))))
    (else
      (Components|StaticMesh|SetStaticMesh (Variables|Default|GetTrims) (Utilities|Array|Get(acopy) (LocalVariables|GetTrim_Meshes_Regular) (Math|Conversions|ToInteger(Byte) (Variables|Customization|GetTrim_Type))))))
  (Rendering|Material|SetMaterial (Variables|Default|GetWall_Corners) 0 (Utilities|Array|Get(acopy) (LocalVariables|GetWall_Materials) (Math|Conversions|ToInteger(Byte) (Variables|Customization|GetWallpaper_Type)))))