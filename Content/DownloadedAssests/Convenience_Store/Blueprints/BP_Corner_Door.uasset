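; A modular corner wall piece with a door for the convenience store environment, configured entirely in the Construction Script.
; Enum settings index mesh and material arrays to pick the wall, trim and wallpaper.
; The corner door type also selects the trim set and, for the second side, moves and rotates the door and frame.
; The metal plate component is destroyed when its option is disabled, and the Event Graph is empty.
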(event EventBeginPlay)

(event Collision|EventActorBeginOverlap
  (params (OtherActor :type Actor%20Object%20Reference)))

(event EventTick
  (params (DeltaSeconds :type Float%20%28single-precision%29)))

(fn ConstructionScript
  (bind _corner_door_type (Variables|Customization|GetCorner_Door_Type))
  (bind _door_frame (Variables|Default|GetDoor_Frame))
  (bind _door (Variables|Default|GetDoor))
  (bind _returnvalue (Math|Conversions|ToInteger(Byte) _corner_door_type))
  (Components|StaticMesh|SetStaticMesh (Variables|Default|GetWall) (Utilities|Array|Get(acopy) (LocalVariables|GetWall_Meshes) _returnvalue))
  (LocalVariables|SetSide_A (== _returnvalue 0))
  (if (LocalVariables|GetSide_A)
    (Components|StaticMesh|SetStaticMesh (Variables|Default|GetDoor_Frame) "/Game/DownloadedAssests/Convenience_Store/Meshes/SM_Door_Frame_C.SM_Door_Frame_C")
    (Components|StaticMesh|SetStaticMesh (Variables|Default|GetDoor) "/Game/DownloadedAssests/Convenience_Store/Meshes/SM_Door.SM_Door")
    (Components|StaticMesh|SetStaticMesh (Variables|Default|GetWall_Trim) (Utilities|Array|Get(acopy) (LocalVariables|GetWall_Trim_Meshes_A) (Math|Conversions|ToInteger(Byte) (Variables|Customization|GetWall_Trim_Type))))
    (else
      (Transformation|SetRelativeLocationAndRotation _door_frame "0.000000,200.000000, 0" "0,90.000000, 0" false false)
      (Components|StaticMesh|SetStaticMesh _door_frame "/Game/DownloadedAssests/Convenience_Store/Meshes/SM_Door_Frame_C.SM_Door_Frame_C")
      (Transformation|SetRelativeLocationAndRotation _door "22.350000,155.800003,107.862640" "0,90.000000, 0" false false)
      (Components|StaticMesh|SetStaticMesh _door "/Game/DownloadedAssests/Convenience_Store/Meshes/SM_Door.SM_Door")
      (Components|StaticMesh|SetStaticMesh (Variables|Default|GetWall_Trim) (Utilities|Array|Get(acopy) (LocalVariables|GetWall_Trim_Meshes_B) (Math|Conversions|ToInteger(Byte) (Variables|Customization|GetWall_Trim_Type))))))
  (Components|StaticMesh|SetStaticMesh (Variables|Default|GetMetal_Plate) "/Game/DownloadedAssests/Convenience_Store/Meshes/SM_Door_Metalplate.SM_Door_Metalplate")
  (Rendering|Material|SetMaterial (Variables|Default|GetWall) 0 (Utilities|Array|Get(acopy) (LocalVariables|GetWallpaper_Materials) (Math|Conversions|ToInteger(Byte) (Variables|Customization|GetWallpaper_Type))))
  (LocalVariables|SetMetalplate_Disabled (== (Math|Conversions|ToInteger(Byte) (Variables|Customization|GetMetalplate)) 0))
  (if (LocalVariables|GetMetalplate_Disabled)
    (Components|DestroyComponent (Variables|Default|GetMetal_Plate))))